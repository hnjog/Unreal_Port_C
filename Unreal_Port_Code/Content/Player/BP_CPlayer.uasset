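; BP_CPlayer is the player Blueprint, and its only active logic toggles the inventory screen through the InInventroy event.
; A FlipFlop alternates between opening a newly created WBP_Inventory and calling Out on the stored widget if it is still valid.
; Opening shows the mouse cursor, sets Game and UI input focused on the widget, and freezes the game with zero global time dilation.
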(event `self.InInventroy`
  (bind _returnvalue (`GameplayStatics.GetPlayerController` 0))
  (bind _invenwidget (`self.InvenWidget`))
  (`/Engine/EditorBlueprintResources/StandardMacros.FlipFlop`
    (:`A`
      (bind _returnvalue_2 (`|CreateWidget` "/Game/Widzets/WBP_Inventory.WBP_Inventory_C" (`GameplayStatics.GetPlayerController` 0)))
      (set `self.InvenWidget` _returnvalue_2)
      (`UserWidget.AddToViewport` _returnvalue_2 0)
      (set `PlayerController.bShowMouseCursor` true _returnvalue)
      (`WidgetBlueprintLibrary.SetInputMode_GameAndUIEx` _returnvalue _returnvalue_2)
      (`GameplayStatics.SetGlobalTimeDilation` 0.0))
    (:`B`
      (`/Engine/EditorBlueprintResources/StandardMacros.IsValid` _invenwidget
        (:`Is Valid`
          (`/Game/Widzets/WBP_Inventory.Out` _invenwidget))))))

(fn `UserConstructionScript`)